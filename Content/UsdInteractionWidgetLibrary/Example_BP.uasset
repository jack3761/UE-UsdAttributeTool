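; Example Blueprint for the USD Interaction Widget Library, showing key-driven playback of a frame range from a UsdStageActor's level sequence.
; L plays the range from a named camera and re-triggers it on the player's OnFinished event for an endless loop, while S stops the current player.
; M repeats it using a loop counter, then switches the view target to another camera.
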(event `Key|L`
  (params (Key :type "Key Structure"))
  ;[1 1 1] Example of an infinite loop of the play frame range from a key press, can be stopped by the stop example below and the stop button
  (:`Pressed`
    (bind _out_camera (`/UsdAttributeTools/UsdInteractionWidgetLibrary/WidgetButtonFunctionLibrary.FindCameraByString` "cameraMain"))
    (bind _returnvalue (`GameplayStatics.GetActorOfClass` "/Script/USDStage.UsdStageActor"))
    (bind _returnvalue_2 (`UsdStageActor.GetLevelSequence` _returnvalue))
    (`/UsdAttributeTools/UsdInteractionWidgetLibrary/WidgetButtonFunctionLibrary.PlayFrameRange` (`GameplayStatics.GetPlayerController` 0) _out_camera 0.0 _returnvalue_2 250 300 :!label _label)
    (bind _level_sequence_player (`/UsdAttributeTools/UsdInteractionWidgetLibrary/WidgetButtonFunctionLibrary.GetLevelSequencePlayer`))
    (add `MovieSceneSequencePlayer.OnFinished` _level_sequence_player (delegate `OnFinished`))))

(event `OnFinished`
  ;[1 1 1] Example of an infinite loop of the play frame range from a key press, can be stopped by the stop example below and the stop button
  (goto _label))

(event `Key|S`
  (params (Key :type "Key Structure"))
  ;[1 1 1] Manual example of how to set a key press to stop the current level sequence player
  (:`Pressed`
    (bind _is_valid (`/UsdAttributeTools/UsdInteractionWidgetLibrary/WidgetButtonFunctionLibrary.IsCurrentSequencePlayer`))
    (if _is_valid
      (bind _level_sequence_player (`/UsdAttributeTools/UsdInteractionWidgetLibrary/WidgetButtonFunctionLibrary.GetLevelSequencePlayer`))
      (`MovieSceneSequencePlayer.Stop` _level_sequence_player))))

(event `Key|M`
  (params (Key :type "Key Structure"))
  ;[1 1 1] Example of how to set up a given number of loops. We use an OnFinished event which is called when the sequence player stops. From here, we have integer variables which can be set on the left, the important one is the loop count, which should be set to 1 initially. We check to see if the loop count is less than the desired number of loops. If it is, we increment the loop count and start again, plauing the sequence and returning to this point. Once the loop count is no longer less than the desired number of loops, we set the camera to the desired one
  (:`Pressed`
    (bind _out_camera (`/UsdAttributeTools/UsdInteractionWidgetLibrary/WidgetButtonFunctionLibrary.FindCameraByString` "cameraMain"))
    (bind _returnvalue (`GameplayStatics.GetActorOfClass` "/Script/USDStage.UsdStageActor"))
    (bind _returnvalue_2 (`UsdStageActor.GetLevelSequence` _returnvalue))
    (`/UsdAttributeTools/UsdInteractionWidgetLibrary/WidgetButtonFunctionLibrary.PlayFrameRange` (`GameplayStatics.GetPlayerController` 0) _out_camera 0.0 _returnvalue_2 250 300 :!label _label_2)
    (bind _level_sequence_player (`/UsdAttributeTools/UsdInteractionWidgetLibrary/WidgetButtonFunctionLibrary.GetLevelSequencePlayer`))
    (add `MovieSceneSequencePlayer.OnFinished` _level_sequence_player (delegate `OnFinished2`))))

(event `OnFinished2`
  ;[1 1 1] Example of how to set up a given number of loops. We use an OnFinished event which is called when the sequence player stops. From here, we have integer variables which can be set on the left, the important one is the loop count, which should be set to 1 initially. We check to see if the loop count is less than the desired number of loops. If it is, we increment the loop count and start again, plauing the sequence and returning to this point. Once the loop count is no longer less than the desired number of loops, we set the camera to the desired one
  (if (< (`self.LoopCount`) (`self.NumberOfLoops`))
    (`/Engine/EditorBlueprintResources/StandardMacros.IncrementInt` (`self.LoopCount`)
      (:`  `
        (goto _label_2)))
    (else
      (bind _out_camera (`/UsdAttributeTools/UsdInteractionWidgetLibrary/WidgetButtonFunctionLibrary.FindCameraByString` "camera1"))
      (`PlayerController.SetViewTargetWithBlend` (`GameplayStatics.GetPlayerController` 0) _out_camera 0.0 "VTBlend_Linear" 0.0 false))))

(fn `UserConstructionScript`)